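; BP_CannonBall is a projectile actor that damages obstacles and ships on impact.
; When its SphereCollision component hits, it casts the other actor to BP_Obstacle, then to BP_Ship, and subtracts Damage directly from that actor's Health.
; The ball destroys itself after damaging either type; hits on any other actor leave it in the world.
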(event `self.ReceiveTick`
  (params (DeltaSeconds :type "Float (single-precision)")))

(event `self.SphereCollision.OnComponentHit`
  (params (HitComponent :type "PrimitiveComponent Object Reference") (OtherActor :type "Actor Object Reference") (OtherComp :type "PrimitiveComponent Object Reference") (NormalImpulse :type "Vector Structure") (Hit :type "HitResult Structure (by ref)"))
  (bind _asbp_obstacle (cast `/Game/Blueprints/Obstacle/BP_Obstacle` OtherActor)
    (:`then`
      (set `/Game/Blueprints/Obstacle/BP_Obstacle.Health` (- (`/Game/Blueprints/Obstacle/BP_Obstacle.Health` _asbp_obstacle) (`self.Damage`)) _asbp_obstacle))
    (:`CastFailed`
      (bind _asbp_ship (cast `/Game/Blueprints/BP_Ship` OtherActor))
      (set `/Game/Blueprints/BP_Ship.Health` (- (`/Game/Blueprints/BP_Ship.Health` _asbp_ship) (`self.Damage`)) _asbp_ship)))
  (`self.K2_DestroyActor`))

(fn `UserConstructionScript`)