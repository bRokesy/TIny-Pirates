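; BP_Cannon is a player-operable cannon that registers itself as the character's nearby cannon while inside its interaction box.
; EnterControl and ExitControl blend the camera and toggle player movement.
; RotateYaw and clamped RotatePitch turn the barrel pivot, though both drive the pitch axis.
; Fire spawns cooldown-limited projectiles at the muzzle, setting local X velocity from the world forward vector's X, with placeholder sound and emitter calls.
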(event `self.InteractionBox.OnComponentBeginOverlap`
  (params (OverlappedComponent :type "PrimitiveComponent Object Reference") (OtherActor :type "Actor Object Reference") (OtherComp :type "PrimitiveComponent Object Reference") (OtherBodyIndex :type Integer) (bFromSweep :type Boolean) (SweepResult :type "HitResult Structure (by ref)"))
  (bind _asbp_third_person_character (cast `/Game/ThirdPerson/Blueprints/BP_ThirdPersonCharacter` OtherActor))
  (set `/Game/ThirdPerson/Blueprints/BP_ThirdPersonCharacter.NearbyCannon` self _asbp_third_person_character))

(event `self.InteractionBox.OnComponentEndOverlap`
  (params (OverlappedComponent :type "PrimitiveComponent Object Reference") (OtherActor :type "Actor Object Reference") (OtherComp :type "PrimitiveComponent Object Reference") (OtherBodyIndex :type Integer))
  (bind _asbp_third_person_character (cast `/Game/ThirdPerson/Blueprints/BP_ThirdPersonCharacter` OtherActor))
  (if (== (`/Game/ThirdPerson/Blueprints/BP_ThirdPersonCharacter.NearbyCannon` _asbp_third_person_character) self)
    (set `/Game/ThirdPerson/Blueprints/BP_ThirdPersonCharacter.NearbyCannon` null _asbp_third_person_character)))

(fn `EnterControl`
  (params (PlayerRef :type "/Game/ThirdPerson/Blueprints/BP_ThirdPersonCharacter Object Reference"))
  (locals (NewLocalVar :type "/Game/ThirdPerson/Blueprints/BP_ThirdPersonCharacter Object Reference"))
  (bind _playerref (`local.PlayerRef`)
    (:`then`
      (set `self.ControllingPlayer` _playerref)
      (set `/Game/ThirdPerson/Blueprints/BP_ThirdPersonCharacter.bControllingCannon` true (`local.PlayerRef`))
      (bind _output_get (set `/Game/ThirdPerson/Blueprints/BP_ThirdPersonCharacter.ControlledCannon` self (`local.PlayerRef`)))
      (set `/Game/Blueprints/BP_Cannon.bIsControlled` true _output_get)
      (`PlayerController.SetViewTargetWithBlend` (`GameplayStatics.GetPlayerController` 0) self 0.5 "VTBlend_Linear" 0.0 false)
      (`CharacterMovementComponent.DisableMovement` (`Character.CharacterMovement` (`local.PlayerRef`)))
      (`Controller.SetIgnoreMoveInput` (`GameplayStatics.GetPlayerController` 0) true))
    (:`else`)))

(fn `ExitControl`
  (bind _controllingplayer (`self.ControllingPlayer`))
  (set `self.bIsControlled` false)
  (`PlayerController.SetViewTargetWithBlend` (`GameplayStatics.GetPlayerController` 0) (`self.ControllingPlayer`) 0.5 "VTBlend_Linear" 0.0 false)
  (`CharacterMovementComponent.SetMovementMode` (`Character.CharacterMovement` (`self.ControllingPlayer`)) "MOVE_Walking" 0)
  (`Controller.SetIgnoreMoveInput` (`GameplayStatics.GetPlayerController` 0) false)
  (set `/Game/ThirdPerson/Blueprints/BP_ThirdPersonCharacter.bControllingCannon` false _controllingplayer)
  (set `/Game/ThirdPerson/Blueprints/BP_ThirdPersonCharacter.ControlledCannon` null _controllingplayer)
  (set `self.ControllingPlayer` null))

(fn `Fire`
  (bind _returnvalue_x (`KismetMathLibrary.BreakVector` (* (`SceneComponent.GetForwardVector` (`self.MuzzlePoint`)) (* (`self.LaunchSpeed`) 1.0))))
  (`self.ProjectileClass`
    (:`then`
      (if (>= (- (`KismetSystemLibrary.GetGameTimeInSeconds`) (`self.LastFireTime`)) (`self.FireCooldown`))
        (set `self.LastFireTime` (`KismetSystemLibrary.GetGameTimeInSeconds`))
        (bind _returnvalue (`|SpawnActorFromClass` (`self.ProjectileClass`) (`SceneComponent.K2_GetComponentToWorld` (`self.MuzzlePoint`)) "Undefined" "MultiplyWithRoot" null null))
        (`ProjectileMovementComponent.SetVelocityInLocalSpace` (`/Game/Blueprints/BP_CannonBall.ProjectileMovement` _returnvalue) (`KismetMathLibrary.MakeVector` _returnvalue_x))
        (`GameplayStatics.PlaySoundAtLocation` "/Engine/EditorSounds/Notifications/CompileFailed.CompileFailed" (0.0 0.0 0.0) (struct) 1.0 1.0 0.0 null null null null)
        (`GameplayStatics.SpawnEmitterAtLocation` null)))
    (:`else`)))

(fn `RotatePitch`
  (params (AxisValue :type "Float (double-precision)"))
  (if (`self.bIsControlled`)
    (`SceneComponent.K2_SetRelativeRotation` (`self.BarrelPivot`) (`KismetMathLibrary.MakeRotator` 0.0 (`KismetMathLibrary.FClamp` (+ (.pitch (`SceneComponent.RelativeRotation` (`self.BarrelPivot`))) (* (* (`local.AxisValue`) (`self.PitchSpeed`)) (`GameplayStatics.GetWorldDeltaSeconds`))) (`self.MinPitch`) (`self.MaxPitch`))) false false)))

(fn `RotateYaw`
  (params (AxisValue :type "Float (double-precision)"))
  (if (`self.bIsControlled`)
    (`SceneComponent.K2_AddLocalRotation` (`self.BarrelPivot`) (`KismetMathLibrary.MakeRotator` 0.0 (* (* (`local.AxisValue`) (`self.YawSpeed`)) (`GameplayStatics.GetWorldDeltaSeconds`))) false false)))

(fn `UserConstructionScript`)