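; BP_Ship is a physics-driven ship that a BP_ThirdPersonCharacter can take control of and sail.
; The steering wheel trigger registers the ship on an overlapping character; its exit check compares the character to the ship, so that reference is never cleared.
; StartControll and StopControll toggle control, and SetShipInput stores throttle and steer.
; While controlled, Tick applies forward or reverse force and yaw torque as accelerations, independent of mass and speed.
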(event `self.ReceiveBeginPlay`
  (`StaticMeshComponent.SetStaticMesh` (`self.ShipMesh`) (`self.BodyShip`)))

(event `self.ReceiveTick`
  (params (DeltaSeconds :type "Float (single-precision)"))
  (if (`self.bIsControlled `)
    (`self.ApplyShipMovement`)
    (`self.RotationShip`)))

(event `self.SteeringWheelTrigger.OnComponentBeginOverlap`
  (params (OverlappedComponent :type "PrimitiveComponent Object Reference") (OtherActor :type "Actor Object Reference") (OtherComp :type "PrimitiveComponent Object Reference") (OtherBodyIndex :type Integer) (bFromSweep :type Boolean) (SweepResult :type "HitResult Structure (by ref)"))
  (bind _asbp_third_person_character (cast `/Game/ThirdPerson/Blueprints/BP_ThirdPersonCharacter` OtherActor))
  (set `/Game/ThirdPerson/Blueprints/BP_ThirdPersonCharacter.CurrentShipToControl` self _asbp_third_person_character)
  (`KismetSystemLibrary.PrintString` "Можно управлять кораблём"))

(event `self.SteeringWheelTrigger.OnComponentEndOverlap`
  (params (OverlappedComponent :type "PrimitiveComponent Object Reference") (OtherActor :type "Actor Object Reference") (OtherComp :type "PrimitiveComponent Object Reference") (OtherBodyIndex :type Integer))
  (bind _asbp_third_person_character (cast `/Game/ThirdPerson/Blueprints/BP_ThirdPersonCharacter` OtherActor))
  (if (== _asbp_third_person_character self)
    (set `/Game/ThirdPerson/Blueprints/BP_ThirdPersonCharacter.CurrentShipToControl` null _asbp_third_person_character)
    (`KismetSystemLibrary.PrintString` "Вышел из зоны штурвала")))

(fn `ApplyShipMovement`
  (`PrimitiveComponent.AddForce` (`self.ShipMesh`) (* (`SceneComponent.GetForwardVector` (`self.ShipMesh`)) (`KismetMathLibrary.SelectFloat` (`self.EngineForce`) (`self.ReverseForce  `) (>= (`self.ThrottleInput `) 0.0)) (`self.ThrottleInput `)) "None" true))

(fn `GetShipCameraActor`)

(fn `RotationShip`
  (bind _returnvalue (`PrimitiveComponent.GetPhysicsLinearVelocity` (`self.ShipMesh`) "None"))
  (`PrimitiveComponent.AddTorqueInDegrees` (`self.ShipMesh`) (`KismetMathLibrary.MakeVector` 0.0 0.0 (* (`self.TurnTorque`) (`self.SteerInput  `) 0.01)) "None" true))

(fn `SetShipInput`
  (params (NewThrottle :type "Float (double-precision)") (NewSteer :type "Float (double-precision)"))
  (set `self.ThrottleInput ` NewThrottle)
  (bind _output_get (set `self.SteerInput  ` NewSteer))
  (`KismetSystemLibrary.PrintString` (`KismetStringLibrary.Conv_DoubleToString` _output_get)))

(fn `StartControll`
  (params (CharacterRef :type "/Game/ThirdPerson/Blueprints/BP_ThirdPersonCharacter Object Reference"))
  (set `self.ControllingCharacter` CharacterRef)
  (set `self.bIsControlled ` true))

(fn `StopControll`
  (set `self.bIsControlled ` false)
  (set `self.ControllingCharacter` null)
  (set `self.ThrottleInput ` 0.0)
  (set `self.SteerInput  ` 0.0))

(fn `UserConstructionScript`)