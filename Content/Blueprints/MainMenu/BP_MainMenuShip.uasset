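; Main menu ship pawn that moves toward a target location supplied through its variables.
; While a target is active, Tick applies movement input toward it and clears the flag within the acceptance radius.
; The mesh's world yaw is taken from the Z component of the mesh-to-target offset, not a look-at angle.
; The 5 key toggles the mouse cursor through a FlipFlop.
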(event `Key|Five`
  (params (Key :type "Key Structure"))
  (bind _returnvalue (`GameplayStatics.GetPlayerController` 0))
  (:`Pressed`
    (`/Engine/EditorBlueprintResources/StandardMacros.FlipFlop`
      (:`A`
        (set `PlayerController.bShowMouseCursor` true _returnvalue))
      (:`B`
        (set `PlayerController.bShowMouseCursor` false _returnvalue)))))

(event `self.ReceiveTick`
  (params (DeltaSeconds :type "Float (single-precision)"))
  (bind _movetargetlocation_location (`KismetMathLibrary.BreakTransform` (`self.MoveTargetLocation`)))
  (bind _movetargetlocation_location_2 (`KismetMathLibrary.BreakTransform` (`self.MoveTargetLocation`)))
  (bind _movetargetlocation_location_3 (`KismetMathLibrary.BreakTransform` (`self.MoveTargetLocation`)))
  (bind (_returnvalue_x _returnvalue_y _returnvalue_z) (`KismetMathLibrary.BreakVector` (- _movetargetlocation_location_2 (`SceneComponent.K2_GetComponentLocation` (`self.StaticMesh`)))))
  (if (`self.HasMoveTarget`)
    (`SceneComponent.K2_SetWorldRotation` (`self.StaticMesh`) (`KismetMathLibrary.MakeRotator` 0.0 0.0 _returnvalue_z) false false)
    (if (> (`KismetMathLibrary.VSize` (- _movetargetlocation_location_3 (`self.K2_GetActorLocation`))) (`self.AcceptanceRadius`))
      (`self.AddMovementInput` (- _movetargetlocation_location (`self.K2_GetActorLocation`)))
      (else
        (set `self.HasMoveTarget` false)))))

(fn `UserConstructionScript`)